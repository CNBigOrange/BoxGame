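; Firework shell actor that flies as a physics projectile with a trail effect and detonates into a burst effect after a set time.
; Construction picks trail and burst Niagara systems from type-to-asset maps using FWSettings, applies their colors, and sets lifespan to detonate time plus a delta.
; Tick aligns rotation to velocity.
; A timer triggers detonation, which activates the burst, stops the trail and disables ticking and physics.
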(event Custom|ShellDetonation
  (Variables|Default|SetisDetonated true)
  (CallFunction|ShellDetonate))

(event EventBeginPlay
  (bind _returnvalue (Utilities|Time|SetTimerbyEvent (delegate Custom|ShellDetonation) (Variables|Default|GetDetonateTime))) ; Set detonate time at shell spawn
  (Variables|Default|SetTimerHandle _returnvalue))

(event EventTick
  (params (DeltaSeconds :type Float%20%28single-precision%29))
  (bind _self self)
  (Transformation|SetActorRotation _self (Math|Conversions|RotationFromXVector (Transformation|GetVelocity _self))) ; Follow trajectory
)

(fn ConstructionScript
  (Actor|SetLifeSpan (+ (Variables|Default|GetDetonateTime) (Variables|Default|GetKillDelta)))
  (CallFunction|ShellInitialize))

(fn ShellDetonate
  (Utilities|FlowControl|Sequence
    (:then_0
      (Components|Activation|Activate (Variables|Default|GetShellVFX) false))
    (:then_1
      (Components|Activation|Deactivate (Variables|Default|GetTrailVFX)) ; Turn off trail
      (Actor|Tick|SetActorTickEnabled false)
      (Physics|SetSimulatePhysics (Variables|Default|GetShellCollider) false))
    (:then_2
      (return))))

(fn ShellInitialize
  (bind _fwsettings (Variables|Default|GetFWSettings))
  (bind _trailvfx (Variables|Default|GetTrailVFX))
  (bind _shellvfx (Variables|Default|GetShellVFX))
  (bind _fwsettings_2 (Variables|Default|GetFWSettings))
  (bind (_shelltype _trailtype _primarycolor _secondarycolor _sparkcolor) (Utilities|Struct|BreakSTRUCT_FW_VFXSettings _fwsettings))
  (bind (_shelltype_2 _trailtype_2) (Utilities|Struct|BreakSTRUCT_FW_VFXSettings _fwsettings_2))
  (Utilities|FlowControl|Sequence
    (:then_0
      (if (Utilities|Enum|NotEqual(Enum) _trailtype_2 "NewEnumerator0")
        (Class|NiagaraComponent|SetAsset _trailvfx (.Value (Utilities|Map|Find (Variables|Default|GetTrailType) _trailtype)) true)
        (Niagara|SetNiagaraVariable(LinearColor) _trailvfx "PrimColor" _primarycolor)
        (Niagara|SetNiagaraVariable(LinearColor) _trailvfx "SecColor" _secondarycolor)
        (Niagara|SetNiagaraVariable(LinearColor) _trailvfx "SparkColor" _sparkcolor)))
    (:then_1
      (if (Utilities|Enum|NotEqual(Enum) _shelltype_2 "NewEnumerator0")
        (Class|NiagaraComponent|SetAsset _shellvfx (.Value (Utilities|Map|Find (Variables|Default|GetShellType) _shelltype)) true)
        (Niagara|SetNiagaraVariable(LinearColor) _shellvfx "PrimColor" _primarycolor)
        (Niagara|SetNiagaraVariable(LinearColor) _shellvfx "SecColor" _secondarycolor)
        (Niagara|SetNiagaraVariable(LinearColor) _shellvfx "SparkColor" _sparkcolor)))
    (:then_2
      (return))))